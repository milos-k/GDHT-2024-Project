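; Player controller for up to four local players in the car game, covering menu car selection, spawning and camera switching.
; ConnecttoGame shows the player's menu overlay and view; next/previous inputs both call ChangeCar with NextPrevious false.
; Ready spawns and possesses the selected car in player-index colour at an index-matched PlayerStart, attaching that player's CineCamera to its spring arm.
; Mapping contexts switch per phase (menu, ready, isometric driving).
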(event Input|EnhancedActionEvents|EnhancedInputActionIA_NextCar
  (params (ActionValue :type Boolean) (ElapsedSeconds :type Float%20%28double-precision%29) (TriggeredSeconds :type Float%20%28double-precision%29) (InputAction :type Input%20Action%20Object%20Reference :default "/Game/Blueprints/Input/Actions/IA_NextCar.IA_NextCar"))
  (Default|ChangeCar (Variables|Default|GetwMainMenu1) (Variables|Default|GetiPlayerIndex) false))

(event Input|EnhancedActionEvents|EnhancedInputActionIA_PreviousCar
  (params (ActionValue :type Boolean) (ElapsedSeconds :type Float%20%28double-precision%29) (TriggeredSeconds :type Float%20%28double-precision%29) (InputAction :type Input%20Action%20Object%20Reference :default "/Game/Blueprints/Input/Actions/IA_PreviousCar.IA_PreviousCar"))
  (Default|ChangeCar (Variables|Default|GetwMainMenu1) (Variables|Default|GetiPlayerIndex) false))

(event Input|EnhancedActionEvents|EnhancedInputActionIA_Ready
  (params (ActionValue :type Boolean) (ElapsedSeconds :type Float%20%28double-precision%29) (TriggeredSeconds :type Float%20%28double-precision%29) (InputAction :type Input%20Action%20Object%20Reference :default "/Game/Blueprints/Input/Actions/IA_Ready.IA_Ready"))
  (bind _returnvalue (PlayerController|LocalPlayerSubsystems|GetEnhancedInputLocalPlayerSubsystem))
  (:Started
    (Utilities|FlowControl|DoOnce false
      (:Completed
        (CallFunction|SpawnandPossess (Variables|Default|GetiPlayerIndex))
        (Variables|Default|SetbReady? true)
        (Input|RemoveMappingContext _returnvalue "/Game/Blueprints/Input/MappingContexts/IMC_Menu.IMC_Menu" "(bIgnoreAllPressedKeysUntilRelease=True,bForceImmediately=False,bNotifyUserSettings=False)")
        (Input|AddMappingContext _returnvalue "/Game/Blueprints/Input/MappingContexts/IMC_Ready.IMC_Ready" 0 "(bIgnoreAllPressedKeysUntilRelease=True,bForceImmediately=False,bNotifyUserSettings=False)")
        (Default|ReadyPlayer (Variables|Default|GetwMainMenu1) (Variables|Default|GetiPlayerIndex))))))

(event Input|EnhancedActionEvents|EnhancedInputActionIA_ToggleCamera
  (params (ActionValue :type Boolean) (ElapsedSeconds :type Float%20%28double-precision%29) (TriggeredSeconds :type Float%20%28double-precision%29) (InputAction :type Input%20Action%20Object%20Reference :default "/Game/Blueprints/Input/Actions/IA_ToggleCamera.IA_ToggleCamera"))
  (bind _returnvalue (Pawn|GetControlledPawn))
  (bind _self self)
  (:Started
    (if (Variables|Default|GetbSwitchCamera)
      (bind _asvehicle_adv_pawn (Utilities|Casting|CastToVehicleAdvPawn _returnvalue))
      (Utilities|FlowControl|FlipFlop
        (:A
          (Variables|/Script/Engine.SpringArmComponent|SetbInheritPitch (Variables|/Game/Blueprints/Vehicles/Default/VehicleAdvPawn.VehicleAdvPawn_C|GetBackSpringArm _asvehicle_adv_pawn) true)
          (Variables|/Script/Engine.SpringArmComponent|SetbInheritRoll (Variables|/Game/Blueprints/Vehicles/Default/VehicleAdvPawn.VehicleAdvPawn_C|GetBackSpringArm _asvehicle_adv_pawn) true)
          (Variables|/Script/Engine.SpringArmComponent|SetbInheritYaw (Variables|/Game/Blueprints/Vehicles/Default/VehicleAdvPawn.VehicleAdvPawn_C|GetBackSpringArm _asvehicle_adv_pawn) true)
          (Game|Player|SetViewTargetwithBlend _self _returnvalue 0.0 "VTBlend_Linear" 0.0 false))
        (:B
          (Variables|/Script/Engine.SpringArmComponent|SetbInheritPitch (Variables|/Game/Blueprints/Vehicles/Default/VehicleAdvPawn.VehicleAdvPawn_C|GetBackSpringArm _asvehicle_adv_pawn) false)
          (Variables|/Script/Engine.SpringArmComponent|SetbInheritRoll (Variables|/Game/Blueprints/Vehicles/Default/VehicleAdvPawn.VehicleAdvPawn_C|GetBackSpringArm _asvehicle_adv_pawn) false)
          (Variables|/Script/Engine.SpringArmComponent|SetbInheritYaw (Variables|/Game/Blueprints/Vehicles/Default/VehicleAdvPawn.VehicleAdvPawn_C|GetBackSpringArm _asvehicle_adv_pawn) false)
          (bind _outactors (Actor|GetAllActorsOfClass "/Script/CinematicCamera.CineCameraActor"))
          (Game|Player|SetViewTargetwithBlend _self (Utilities|Array|Get(acopy) _outactors (Variables|Default|GetiPlayerIndex)) 0.0 "VTBlend_Linear" 0.0 false)
          (Transformation|SetRelativeRotation (Variables|/Game/Blueprints/Vehicles/Default/VehicleAdvPawn.VehicleAdvPawn_C|GetBackSpringArm _asvehicle_adv_pawn) "90.000000,0.000000,0.000000" false false))))))

(event EventTick
  (params (DeltaSeconds :type Float%20%28single-precision%29)))

(event EventBeginPlay
  ;[1 1 1] BeginPlay Logic
  (Input|SetInputModeGameandUI self 0 "DoNotLock" true false)
  (bind _asgm_car_game_new (Utilities|Casting|CastToGM_CarGame_new (Game|GetGameMode)))
  (Variables|Default|SetwMainMenu1 (Variables|/Game/Blueprints/GameRules/GM_CarGame_new.GM_CarGame_new_C|GetwMainMenu_1 _asgm_car_game_new)))

(event EventStartGame
  (bind _self self)
  ;[1 1 1] ovde je bio problem
  (Input|AddMappingContext (PlayerController|LocalPlayerSubsystems|GetEnhancedInputLocalPlayerSubsystem) "/Game/Blueprints/Input/MappingContexts/IMC_Isometric.IMC_Isometric" 0 "(bIgnoreAllPressedKeysUntilRelease=True,bForceImmediately=False,bNotifyUserSettings=False)")
  (Input|SetInputModeGameOnly _self false)
  (Variables|Default|SetbShowMouseCursor _self false))

(event EventConnecttoGame
  (params (PlayerIndex :type Integer))
  (Variables|Default|SetiPlayerIndex PlayerIndex)
  (Input|AddMappingContext (PlayerController|LocalPlayerSubsystems|GetEnhancedInputLocalPlayerSubsystem) "/Game/Blueprints/Input/MappingContexts/IMC_Menu.IMC_Menu" 0 "(bIgnoreAllPressedKeysUntilRelease=True,bForceImmediately=False,bNotifyUserSettings=False)")
  (Utilities|SetOverlayEnabled (Variables|Default|GetiPlayerIndex))
  (bind _outactors (Actor|GetAllActorsOfClass "/Script/CinematicCamera.CineCameraActor"))
  (Utilities|IsValid (Utilities|Array|Get(acopy) _outactors (Variables|Default|GetiPlayerIndex))
    (:Is%20Valid
      (Game|Player|SetViewTargetwithBlend (Utilities|Array|Get(acopy) _outactors (Variables|Default|GetiPlayerIndex)) 0.0 "VTBlend_Linear" 0.0 false)
      (Transformation|AttachComponentToComponent (Utilities|Array|Get(acopy) _outactors (Variables|Default|GetiPlayerIndex)) 0 "None" "KeepWorld" "KeepWorld" "KeepWorld" true))))

(fn ConstructionScript)

(fn SpawnandPossess
  (params (Player%20Index :type Integer))
  (bind _self self)
  (bind _wmainmenu1 (Variables|Default|GetwMainMenu1))
  (bind _icartypes (Variables|/Game/UI/W_MainMenu_1.W_MainMenu_1_C|GetiCarTypes _wmainmenu1))
  (bind _output (Utilities|Array|Get(acopy) _icartypes Player%20Index))
  (bind _outactors (Actor|GetAllActorsOfClass "/Script/Engine.PlayerStart"))
  (Development|PrintString "player index" true true "(R=0.000000,G=0.660000,B=1.000000,A=1.000000)" 1e+01)
  (Development|PrintString (Utilities|String|ToString(Integer) Player%20Index) true true "(R=0.000000,G=0.660000,B=1.000000,A=1.000000)" 1e+01)
  (Utilities|GetCarClass _output Player%20Index
    (:then
      (Utilities|SetCarColor Player%20Index _output)
      (bind _returnvalue (Game|SpawnActorfromClass (Variables|Default|GetcCarClass) (Transformation|GetActorTransform (Utilities|Array|Get(acopy) _outactors Player%20Index)) "Undefined" "MultiplyWithRoot" 0 (Variables|Default|GetmTeamColor) 0 0))
      (Pawn|Possess _self _returnvalue)
      (bind _outactors_2 (Actor|GetAllActorsOfClass "/Script/CinematicCamera.CineCameraActor"))
      (Utilities|IsValid (Utilities|Array|Get(acopy) _outactors_2 Player%20Index)
        (:Is%20Valid
          (Game|Player|SetViewTargetwithBlend _self (Utilities|Array|Get(acopy) _outactors_2 Player%20Index) 0.0 "VTBlend_Linear" 0.0 false)
          (Transformation|AttachComponentToComponent (Utilities|Array|Get(acopy) _outactors_2 Player%20Index) (Variables|/Game/Blueprints/Vehicles/Default/VehicleAdvPawn.VehicleAdvPawn_C|GetBackSpringArm (.AsVehicle%20Adv%20Pawn (Utilities|Casting|CastToVehicleAdvPawn (Pawn|GetControlledPawn)))) "None" "KeepWorld" "KeepWorld" "KeepWorld" true))))))