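; BP_Coin_Daisy is a coin pickup for vehicle pawns.
; When a VehicleAdvPawn overlaps its box collision, it increments that pawn's HowManyCoins, plays a confirmation sound and destroys itself.
; Two helper functions, WhoCollectedMe? and WhoWon?, match color substrings in a material name to one of four players, yielding an index or win message.
; The event graph calls neither helper.
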(event OnComponentBeginOverlap(BoxCollision)
  (params (OverlappedComponent :type Primitive%20Component%20Object%20Reference) (OtherActor :type Actor%20Object%20Reference) (OtherComp :type Primitive%20Component%20Object%20Reference) (OtherBodyIndex :type Integer) (bFromSweep :type Boolean) (SweepResult :type Hit%20Result%20Structure%20%28by%20ref%29))
  (bind _asvehicle_adv_pawn (Utilities|Casting|CastToVehicleAdvPawn OtherActor))
  (Variables|/Game/Blueprints/Vehicles/Default/VehicleAdvPawn.VehicleAdvPawn_C|Sethow_many_coins _asvehicle_adv_pawn (+ (Variables|/Game/Blueprints/Vehicles/Default/VehicleAdvPawn.VehicleAdvPawn_C|Gethow_many_coins _asvehicle_adv_pawn) 1))
  (Audio|PlaySound2D "/Game/UI/Sounds/confirmation_001.confirmation_001" 1.0 1.0 0.0 0 0)
  (Actor|DestroyActor))

(fn ConstructionScript)